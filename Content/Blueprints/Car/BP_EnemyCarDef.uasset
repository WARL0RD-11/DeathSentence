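; BP_EnemyCarDef is an enemy car Blueprint that still carries player-style vehicle input handling.
; Thumbstick and touch events forward to Do* functions for steering, throttle, braking, handbrake, look-around, camera toggle and reset, with a Braking flag firing brake start and stop once per change.
; Headlight input and touch share a FlipFlop that toggles both lights' visibility.
; BeginPlay stores the start location; no AI logic appears in the graph.
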(event `self.ReceiveBeginPlay`
  (set `self.StartLocation` (`self.K2_GetActorLocation`)))

(event `self.Primary Thumbstick`
  (params (Axis :type "Vector2D Structure"))
  (bind _braking (`self.Braking`))
  ; Input Management for Vehicle Pawn
  (`self.DoSteering` Axis_X)
  (if (>= Axis_Y 0.0)
    (`self.DoThrottle` Axis_Y)
    (if _braking
      (set `self.Braking` false)
      (`self.DoBrakeStop`))
    (else
      (`self.DoBrake` (* Axis_Y -1.0))
      (if (not _braking)
        (set `self.Braking` true)
        (`self.DoBrakeStart`)))))

(event `self.Secondary Thumbstick`
  (params (Axis :type "Vector2D Structure"))
  ; Input Management for Vehicle Pawn
  (`self.DoLookAround` Axis_X))

(event `EnhancedInput|/Game/VehicleTemplate/Input/Actions/IA_Headlights`
  (params (ActionValue :type Boolean) (ElapsedSeconds :type "Float (double-precision)") (TriggeredSeconds :type "Float (double-precision)") (InputAction :type "InputAction Object Reference" :default "/Game/VehicleTemplate/Input/Actions/IA_Headlights.IA_Headlights"))
  ; Input Management for Vehicle Pawn
  (:`Triggered`
    (bind _isa (`/Engine/EditorBlueprintResources/StandardMacros.FlipFlop` :!label _label)
      (:`A`
        _)
      (:`B`
        _))
    (`SceneComponent.SetVisibility` (`self.Headlight_L`) _isa false)
    (`SceneComponent.SetVisibility` (`self.Headlight_R`) _isa false)))

(event `self.Touch Headlights `
  ; Input Management for Vehicle Pawn
  (goto _label))

(event `self.Touch Handbrake Start`
  ; Input Management for Vehicle Pawn
  (`self.DoHandbrakeStart`))

(event `self.Touch Handbrake End`
  ; Input Management for Vehicle Pawn
  (`self.DoHandbrakeStop`))

(event `self.Touch Reset`
  ; Input Management for Vehicle Pawn
  (`self.DoResetVehicle`))

(event `self.Touch Toggle Camera`
  ; Input Management for Vehicle Pawn
  (`self.DoToggleCamera`))

(fn `UserConstructionScript`)